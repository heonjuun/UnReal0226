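; Monster pawn with a rough chase-or-return-home behavior driven by AI MoveTo.
; A single distance check on BeginPlay targets the player when the distance is at least DetectRadius, otherwise HomeLocation with DetectRadius as acceptance radius.
; The logic looks unfinished: the distance check has no target actor, the chase move has no pawn set, and its follow-up movement input is a zero vector.
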(event EventBeginPlay
  (if (>= (Transformation|GetDistanceTo (Game|GetPlayerCharacter 0) 0) (Variables|Default|GetDetectRadius))
    (AI|AIMoveTo 0 (- (Transformation|GetDistanceTo (Game|GetPlayerCharacter 0) 0) (Transformation|GetActorLocation)) (Game|Player|GetPlayerPawn 0) 0.0 false
      (:then
        (Pawn|Input|AddMovementInput "0, 0, 0" 1.0 false)))
    (else
      (AI|AIMoveTo self (Variables|Default|GetHomeLocation) 0 (Variables|Default|GetDetectRadius) false))))

(fn ConstructionScript)