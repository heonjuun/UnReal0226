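; BP_Test2 is a test actor that sways side to side along its root component's right vector.
; Each Tick adds delta time to RunnigTime, feeds it through a sine scaled by MoveSpeed and MoveDistance, and sets the location to Start plus that offset without sweeping.
; The graphs never assign Start, so the center of the motion comes from that variable's existing value.
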(event EventTick
  (params (DeltaSeconds :type Float%20%28single-precision%29))
  ;[0.15 0.15 0.15 0.5] 시간누적
  (bind _output_get (Variables|Default|SetRunnigTime (+ DeltaSeconds (Variables|Default|GetRunnigTime))))
  (Transformation|SetActorLocation (+ (Variables|Default|GetStart) (* (Math|Vector|GetRightVector (Variables|Default|GetDefaultSceneRoot)) (* (Math|Trig|Sin(Radians) (* _output_get (Variables|Default|GetMoveSpeed))) (Variables|Default|GetMoveDistance)))) false false))

(fn ConstructionScript)