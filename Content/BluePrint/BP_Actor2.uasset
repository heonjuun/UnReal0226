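; BP_Actor2 is an actor that constantly moves forward and rolls its static mesh in response to player input.
; Tick offsets its location along the forward vector by Speed and delta time, without sweeping for collision.
; The Turn input axis applies a frame-rate-scaled local roll to the mesh, using the Turn variable as the rate and skipping it when that is zero.
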(event EventTick
  (params (DeltaSeconds :type Float%20%28single-precision%29))
  (Transformation|SetActorLocation (+ (Transformation|GetActorLocation) (* (Transformation|GetActorForwardVector) (* DeltaSeconds (Variables|Default|GetSpeed)))) false false))

(event EventBeginPlay)

(event Input|AxisEvents|InputAxisTurn
  (params (AxisValue :type Float%20%28single-precision%29))
  (if (!= (Variables|Default|GetTurn) 0.0)
    (Transformation|AddLocalRotation (Variables|Default|GetStaticMesh) (Math|Rotator|MakeRotator (* (* AxisValue (Utilities|Time|GetWorldDeltaSeconds)) (Variables|Default|GetTurn)) 0.0 0.0) false false)))

(fn ConstructionScript)