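; Door actor Blueprint that opens and closes through its DoorOpen and DoorClose events, which are not called within this graph.
; One Timeline drives both directions, playing to swing Pivot from 0 to 90 degrees yaw while sliding BallController along local Y, and reversing to close.
; ForwardBox overlap events toggle an IsForwardBox flag, which nothing in this graph reads.
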(event OnComponentBeginOverlap(ForwardBox)
  (params (OverlappedComponent :type Primitive%20Component%20Object%20Reference) (OtherActor :type Actor%20Object%20Reference) (OtherComp :type Primitive%20Component%20Object%20Reference) (OtherBodyIndex :type Integer) (bFromSweep :type Boolean) (SweepResult :type Hit%20Result%20Structure%20%28by%20ref%29))
  (Variables|Default|SetIsForwardBox true))

(event OnComponentEndOverlap(ForwardBox)
  (params (OverlappedComponent :type Primitive%20Component%20Object%20Reference) (OtherActor :type Actor%20Object%20Reference) (OtherComp :type Primitive%20Component%20Object%20Reference) (OtherBodyIndex :type Integer))
  (Variables|Default|SetIsForwardBox false))

(event Custom|DoorOpen
  (bind _open (Timeline|Timeline Play)
    (:Update
      (Transformation|SetRelativeRotation (Variables|Default|GetPivot) (Math|Rotator|MakeRotator 0.0 0.0 (Math|Float|Lerp 0.0 9e+01 _open)) false false)
      (Transformation|SetRelativeLocation (Variables|Default|GetBallController) (Math|Vector|MakeVector 0.0 (Math|Float|Lerp 0.0 9e+01 _open) 0.0) false false))))

(event Custom|DoorClose
  (bind _open (Timeline|Timeline Reverse)
    (:Update
      (Transformation|SetRelativeRotation (Variables|Default|GetPivot) (Math|Rotator|MakeRotator 0.0 0.0 (Math|Float|Lerp 0.0 9e+01 _open)) false false)
      (Transformation|SetRelativeLocation (Variables|Default|GetBallController) (Math|Vector|MakeVector 0.0 (Math|Float|Lerp 0.0 9e+01 _open) 0.0) false false))))

(fn ConstructionScript)