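; BP_Actor is an airplane actor that flies forward continuously and prints its name on BeginPlay.
; Tick moves it along the actor's forward vector by MoveSpeed scaled by delta time, setting location directly without sweep for frame-rate-independent motion.
; The Turn input axis adds local pitch rotation to the StaticMesh, scaled by Rotation and world delta time.
; Two fixed-step pitch rotation nodes remain unconnected.
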(event EventBeginPlay
  (Development|PrintString "BP_Airplane"))

(event EventTick
  (params (DeltaSeconds :type Float%20%28single-precision%29))
  ;[0.15 0.15 0.15 0.5] 컴퓨터 성능의 차이로 인한 프레임수가달라져도, 실제 시간 기준으로는 속도를 일정하게 맞춰주는 보정값
  ;;[0.15 0.15 0.15 0.5] Delta=이전 프레임으로 부터 현재 프레임까지 걸린 시간
  ;;[0.15 0.15 0.15 0.5] NEw Location 위치로 좌표 강제이동
  (Transformation|SetActorLocation (+ (Transformation|GetActorLocation) (* (Transformation|GetActorForwardVector) (* DeltaSeconds (Variables|Default|GetMoveSpeed)))) false false))

(event Input|AxisEvents|InputAxisTurn
  (params (AxisValue :type Float%20%28single-precision%29))
  (bind _returnvalue (Utilities|Time|GetWorldDeltaSeconds))
  (bind _rotation (Variables|Default|GetRotation))
  (bind _returnvalue_2 (* _rotation _returnvalue))
  (if (!= _returnvalue_2 0.0)
    (Transformation|AddLocalRotation (Variables|Default|GetStaticMesh) (Math|Rotator|MakeRotator 0.0 (* AxisValue _returnvalue_2) 0.0) false false)))

(fn ConstructionScript)