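; Test function library of integer addition exercises, each built with a different looping technique.
; Add sums every value from Num11 through Num22 with a for loop.
; Myadd2 loops back on itself, adding Num1 to a local total until it reaches at least 447.
; Myadd3 computes the inclusive range sum recursively, returning zero when the start exceeds the end.
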(fn Add
  (params (num11 :type Integer) (num22 :type Integer))
  ;[0.15 0.15 0.15 0.5] function(함수) x=매개변수,y=출력 input,output
  (for _index (range num11 num22)
    (LocalVariables|SetTemp (+ _index (LocalVariables|GetTemp))))
  (return (LocalVariables|GetTemp)))

(fn Myadd2
  (params (Num1 :type Integer))
  (bind _output_get (LocalVariables|SetTemp (stale _output_get_2)))
  (if (>= (LocalVariables|GetTemp) 447) :!label _label
    (return _output_get)
    (else
      (bind _output_get_2 (LocalVariables|SetTemp (+ Num1 (LocalVariables|GetTemp))))
      (goto _label))))

(fn Myadd3
  (params (num1 :type Integer) (num2 :type Integer))
  (if (> num1 num2)
    (return 0)
    (elif (== num1 num2)
      (return num1)
      (else
        (bind _sum (CallFunction|Myadd3 (+ num1 1) num2))
        (LocalVariables|SetTemp _sum)
        (return (+ num1 (LocalVariables|GetTemp)))))))