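; AttackTrap is a trap actor that swings back and forth along its root component's right vector.
; Tick accumulates running time and sets the location to StartLocation plus a sine offset scaled by MoveSpeed and MoveDistance, without sweeping.
; The graphs only read StartLocation, never set it, and contain no attack, damage or overlap logic.
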(event EventTick
  (params (DeltaSeconds :type Float%20%28single-precision%29))
  (bind _output_get (Variables|Default|SetRunningTime (+ DeltaSeconds (Variables|Default|GetRunningTime))))
  (Transformation|SetActorLocation (+ (Variables|Default|GetStartLocation) (* (Math|Vector|GetRightVector (Variables|Components|GetDefaultSceneRoot)) (* (Math|Trig|Sin(Radians) (* _output_get (Variables|Default|GetMoveSpeed))) (Variables|Default|GetMoveDistance)))) false false))

(fn ConstructionScript)