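; BP_Aim is a HUD Blueprint that draws a crosshair at the center of the screen.
; DrawHUD runs each frame and draws the Cross_Hair texture at a fixed size, offset by half that size from the screen midpoint to center it.
; On BeginPlay it also creates WBP_TestWidget, passes it the 검3 image through UpdateImage and adds it to the viewport.
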(event EventBeginPlay
  (bind _returnvalue (UserInterface|CreateWidget "/Game/Test/WBP_TestWidget.WBP_TestWidget_C"))
  (Default|UpdateImage _returnvalue "/Game/Test/검3.검3")
  (UserInterface|Viewport|AddtoViewport _returnvalue 0))

(event EventDrawHUD
  (params (SizeX :type Integer) (SizeY :type Integer))
  ;[0.15 0.15 0.15 0.5] 화면의 크기를 전달해줌(허드에 화면크기를 알려주는 리시브 드로우 허드 함수 제공) 매 프레임마다 실행되는 구조
  ;[0.15 0.15 0.15 0.5] 화면의 x좌표 y좌표에 텍스쳐 표기만
  (Canvas|DrawTexture "/Game/Assets/Cross_Hair.Cross_Hair" (Math|Conversions|ToFloat(Integer) (- (/ SizeX 2) 24)) (Math|Conversions|ToFloat(Integer) (- (/ SizeY 2) 24)) 48.0 48.0 0.0 0.0 1.0 1.0 "(R=1.000000,G=1.000000,B=1.000000,A=1.000000)"))

(fn ConstructionScript)