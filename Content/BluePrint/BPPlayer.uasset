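; Player character Blueprint for an FPS-style game with balloon shooting, a melee-style attack and item pickups.
; Fire spends ammo, plays a montage and line-traces from the deprojected screen center, calling Boom on any hit BP_Balloon.
; OnPickUpItem copies a DT_ItemData row's stats to the player and updates the BP_Aim HUD's widget with its image and values.
; Attack only plays a montage, OpenDoor is empty, and the event graph holds debug prints.
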(event OnComponentHit(Mesh)
  (params (HitComponent :type Primitive%20Component%20Object%20Reference) (OtherActor :type Actor%20Object%20Reference) (OtherComp :type Primitive%20Component%20Object%20Reference) (NormalImpulse :type Vector :default "0, 0, 0") (Hit :type Hit%20Result%20Structure%20%28by%20ref%29))
  ;[0.15 0.15 0.15 0.5] 회전
  (Development|PrintString "player hit"))

(event OnComponentBeginOverlap(Mesh)
  (params (OverlappedComponent :type Primitive%20Component%20Object%20Reference) (OtherActor :type Actor%20Object%20Reference) (OtherComp :type Primitive%20Component%20Object%20Reference) (OtherBodyIndex :type Integer) (bFromSweep :type Boolean) (SweepResult :type Hit%20Result%20Structure%20%28by%20ref%29))
  ;[0.15 0.15 0.15 0.5] 회전
  (Development|PrintString "start"))

(event OnComponentEndOverlap(Mesh)
  (params (OverlappedComponent :type Primitive%20Component%20Object%20Reference) (OtherActor :type Actor%20Object%20Reference) (OtherComp :type Primitive%20Component%20Object%20Reference) (OtherBodyIndex :type Integer))
  (Development|PrintString "end"))

(event EventBeginPlay
  (bind _returnvalue (Class|DataTableFunctionLibrary|DoesDataTableRowExist "/Game/Test/DT_ItemData.DT_ItemData" "Item1"))
  (Development|PrintString (Utilities|String|ToString(Boolean) _returnvalue)))

(fn ConstructionScript)

(fn Fire
  (bind _returnvalue (Viewport|GetViewportSize))
  (bind _returnvalue_2 (Game|GetPlayerController 0))
  (bind _returnvalue_3 (/ (.y _returnvalue) 2.0))
  (bind _returnvalue_4 (/ (.x _returnvalue) 2.0))
  (bind (_worldposition _worlddirection) (Class|GameplayStatics|DeprojectScreentoWorld _returnvalue_2 (Math|Vector2D|MakeVector2D _returnvalue_4 _returnvalue_3)))
  (if (> (Variables|Default|GetMoCount) 0)
    (Math|Integer|DecrementInt (Variables|Default|GetMoCount)
      (:%20%20
        (Animation|PlayAnimMontage "/Game/animations/Am_Fire.Am_Fire" 1.0 "Default")
        (bind _outhit (Collision|LineTraceByChannel _worldposition (+ (* _worlddirection 5e+03) _worldposition) "TraceTypeQuery1" false 0 "ForDuration"))
        (bind _asbp_balloon (Utilities|Casting|CastToBP_Balloon (.HitActor (Collision|BreakHitResult _outhit))))
        (Default|Boom _asbp_balloon)))))

(fn Attack
  (Animation|PlayAnimMontage "/Game/animations/Attack.Attack" 1.0 "Default"))

(fn OpenDoor)

(fn OnPickUpItem
  (params (RowName :type Name))
  (bind _testwidget (Variables|Default|GetTestWidget))
  (bind _returnvalue (Utilities|GetDataTableRow "/Game/Test/DT_ItemData.DT_ItemData" RowName)
    (:then
      (LocalVariables|SetOutRow _returnvalue)
      (Utilities|FlowControl|Sequence
        (:then_0
          (Variables|Default|SetSpeed (.speed (LocalVariables|GetOutRow)))
          (Variables|Default|SetAttack2 (.attack (LocalVariables|GetOutRow)))
          (Variables|Default|SetLuck (.luck (LocalVariables|GetOutRow))))
        (:then_1
          (Utilities|Casting|CastToBP_Aim (HUD|GetHUD (Game|GetPlayerController 0)))
          (Default|UpdateImage _testwidget (.itemimage (LocalVariables|GetOutRow)))
          (Default|UpdateText _testwidget (Utilities|Text|ToText(Integer) (.speed (LocalVariables|GetOutRow))) (Utilities|Text|ToText(Integer) (.attack (LocalVariables|GetOutRow))) (Utilities|Text|ToText(Integer) (.luck (LocalVariables|GetOutRow)))))))))