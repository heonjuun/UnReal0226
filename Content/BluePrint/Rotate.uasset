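; Actor Blueprint that continuously swings its own rotation back and forth.
; Each Tick accumulates running time and drives a sine wave scaled by MoveSpeed and MoveDistance.
; The wave offsets the Rotate vector along the root component's current right vector, and the result becomes the actor's forward direction through RotationFromXVector.
; The right vector is re-read every frame, so each new rotation feeds into the next.
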(event EventBeginPlay)

(event EventTick
  (params (DeltaSeconds :type Float%20%28single-precision%29))
  (bind _output_get (Variables|Default|SetRunnigTime (+ DeltaSeconds (Variables|Default|GetRunnigTime))))
  (Transformation|SetActorRotation (Math|Conversions|RotationFromXVector (+ (Variables|Default|GetRotate) (* (Math|Vector|GetRightVector (Variables|Default|GetDefaultSceneRoot)) (* (Math|Trig|Sin(Radians) (* _output_get (Variables|Default|GetMoveSpeed))) (Variables|Default|GetMoveDistance)))))))

(fn ConstructionScript)